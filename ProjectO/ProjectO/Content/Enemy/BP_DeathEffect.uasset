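; BP_DeathEffect is an enemy death effect actor that shatters a geometry collection and cleans itself up.
; On BeginPlay it applies a radial velocity-change impulse from the ImpulseLocation component, then removes the Sphere component about a frame later.
; After two seconds it swaps the debris to a glow material for a brief flash before destroying the actor.
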(event `self.ReceiveBeginPlay`
  (`|ExecutionSequence`
    (:`then_0`
      (`PrimitiveComponent.AddRadialImpulse` (`self.GeometryCollection`) (`SceneComponent.K2_GetComponentLocation` (`self.Impulse Location`)) 650.0 2000.0 "RIF_Constant" true))
    (:`then_1`
      (`KismetSystemLibrary.Delay` 0.016)
      (`ActorComponent.K2_DestroyComponent` (`self.Sphere`)))
    (:`then_2`
      (`KismetSystemLibrary.Delay` 2.0)
      (`PrimitiveComponent.SetMaterial` (`self.GeometryCollection`) 0 "/Game/Variant_TwinStick/M_Glow.M_Glow")
      (`KismetSystemLibrary.Delay` 0.16)
      (`self.K2_DestroyActor`))))

(fn `UserConstructionScript`)